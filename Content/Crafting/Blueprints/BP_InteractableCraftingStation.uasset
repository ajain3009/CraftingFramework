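; Interactable crafting station actor that shows a world-space prompt telling the nearby player whether its recipe can be crafted.
; Entering the proximity trigger registers the station on the third-person character, runs the crafting component's CanCraft and builds the prompt from its result.
; Leaving clears that reference, hides the prompt and closes the crafting UI.
; While the player is in range, Tick turns the widget toward the camera.
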(event OnComponentBeginOverlap(ProximityTrigger)
  (params (OverlappedComponent :type Primitive%20Component%20Object%20Reference) (OtherActor :type Actor%20Object%20Reference) (OtherComp :type Primitive%20Component%20Object%20Reference) (OtherBodyIndex :type Integer) (bFromSweep :type Boolean) (SweepResult :type Hit%20Result%20Structure%20%28by%20ref%29))
  (bind _self self)
  (bind _widget (Variables|Default|GetWidget))
  (bind _asbp_third_person_character (Utilities|Casting|CastToBP_ThirdPersonCharacter OtherActor))
  (Utilities|IsValid _asbp_third_person_character
    (:Is%20Valid
      (Variables|/Game/ThirdPerson/Blueprints/BP_ThirdPersonCharacter.BP_ThirdPersonCharacter_C|SetNearbyCraftingStation _asbp_third_person_character _self)
      (bind (_messagetype _outerror _returnvalue) (Class|UCraftingComponent|CanCraft (Variables|/Game/ThirdPerson/Blueprints/BP_ThirdPersonCharacter.BP_ThirdPersonCharacter_C|GetBP_CraftingComponent _asbp_third_person_character) (Variables|/Script/Mawforged.UCraftingStationComponent|GetRecipe (Variables|Default|GetUCraftingStation)) _self))
      (Variables|Default|SetbPlayerInRange true)
      (Variables|Default|SetCraftItem _returnvalue)
      (bind _returnvalue_2 (UserInterface|CreateWidget "/Game/Crafting/Widgets/WBP_InteractionPrompt.WBP_InteractionPrompt_C" 0 _outerror _messagetype))
      (UserInterface|SetWidget _widget _returnvalue_2)
      (Variables|Default|SetCraftingWidgetObject _returnvalue_2)
      (Development|SetHiddeninGame _widget false false))))

(event OnComponentEndOverlap(ProximityTrigger)
  (params (OverlappedComponent :type Primitive%20Component%20Object%20Reference) (OtherActor :type Actor%20Object%20Reference) (OtherComp :type Primitive%20Component%20Object%20Reference) (OtherBodyIndex :type Integer))
  (bind _craftingwidgetobject (Variables|Default|GetCraftingWidgetObject))
  (bind _asbp_third_person_character (Utilities|Casting|CastToBP_ThirdPersonCharacter OtherActor))
  (Utilities|IsValid _asbp_third_person_character
    (:Is%20Valid
      (Variables|/Game/ThirdPerson/Blueprints/BP_ThirdPersonCharacter.BP_ThirdPersonCharacter_C|SetNearbyCraftingStation _asbp_third_person_character 0)
      (Variables|Default|SetbPlayerInRange false)
      (Development|SetHiddeninGame (Variables|Default|GetWidget) true true)
      (Utilities|IsValid _craftingwidgetobject
        (:Is%20Valid
          (Widget|RemovefromParent _craftingwidgetobject)
          (Widget|RemovefromParent (Variables|/Game/ThirdPerson/Blueprints/BP_CraftingComponent.BP_CraftingComponent_C|GetCraftingUIWidget (Variables|/Game/ThirdPerson/Blueprints/BP_ThirdPersonCharacter.BP_ThirdPersonCharacter_C|GetBP_CraftingComponent _asbp_third_person_character))))))))

(event EventBeginPlay)

(event Collision|EventActorBeginOverlap
  (params (OtherActor :type Actor%20Object%20Reference)))

(event EventTick
  (params (DeltaSeconds :type Float%20%28single-precision%29))
  (bind _widget (Variables|Default|GetWidget))
  (if (Variables|Default|GetbPlayerInRange)
    (Transformation|SetRelativeRotation _widget (Math|Rotator|FindLookatRotation (Transformation|GetWorldLocation _widget) (Transformation|GetWorldLocation (Variables|/Script/Engine.PlayerCameraManager|GetTransformComponent (Game|GetPlayerCameraManager 0)))) false false)))

(fn ConstructionScript)

(fn HideCrafingWidget
  (Utilities|IsValid (Variables|Default|GetCraftingWidgetObject)
    (:Is%20Valid
      (Development|SetHiddeninGame (Variables|Default|GetWidget) true false))))

(fn ShowCraftingWidget
  (params (PlayerCraftingComponent :type BP%20Crafting%20Component%20Object%20Reference))
  (bind _widget (Variables|Default|GetWidget))
  (if (Variables|Default|GetbPlayerInRange)
    (bind (_messagetype _outerror _returnvalue) (Class|UCraftingComponent|CanCraft PlayerCraftingComponent (Variables|/Script/Mawforged.UCraftingStationComponent|GetRecipe (Variables|Default|GetUCraftingStation)) self))
    (Variables|Default|SetCraftItem _returnvalue)
    (bind _returnvalue_2 (UserInterface|CreateWidget "/Game/Crafting/Widgets/WBP_InteractionPrompt.WBP_InteractionPrompt_C" 0 _outerror _messagetype))
    (UserInterface|SetWidget _widget _returnvalue_2)
    (Variables|Default|SetCraftingWidgetObject _returnvalue_2)
    (Development|SetHiddeninGame _widget false false)))